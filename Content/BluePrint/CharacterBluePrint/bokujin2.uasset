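; Enemy Blueprint (bokujin2) that targets player 0 and appears to teach attack telegraphs, using cast names as Japanese hints.
; Koudou cycles by action count modulo four through a plain cast, a delayed knockback Rakuseki AoE, and a Kensasi attack described as proximity-damage, leaving the fourth step empty.
; Separate events spawn an ATK-scaled Firemahou (zangeki) or a small delayed Rakuseki (kuromahou).
; Zikkou is empty and its Eisyounum dispatch is disconnected.
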(event `self.zikkou`)

(event `kuromahou`
  (`|SpawnActorFromClass` :`Class` "/Game/BluePrint/gimic/boss1gimic/rakuseki.rakuseki_C" :`SpawnTransform` (`KismetMathLibrary.MakeTransform` (`self.K2_GetActorLocation` (`self.TARGET`))) :`CollisionHandlingOverride` "AlwaysSpawn" :`TransformScaleMethod` "MultiplyWithRoot" :`AoEDamage` 1.0 :`yochoudelay` 8.0 :`Size` 20.0 :`SphereAoE` true :`Instigator` null))

(event `self.ReceiveBeginPlay`
  (`parent.ReceiveBeginPlay`)
  (set `self.TARGET` (`GameplayStatics.GetPlayerCharacter` 0)))

(event `zangeki`
  (`|SpawnActorFromClass` "/Game/BluePrint/firemahou.firemahou_C" (`self.GetTransform`) "AlwaysSpawn" "MultiplyWithRoot" null (* (`KismetMathLibrary.Conv_IntToDouble` (`self.ATK`)) 1.25) (`self.TARGET`) 0.0 null))

(event `self.koudou`
  (bind _koudousuu (`self.koudousuu`))
  (bind _returnvalue (`self.K2_GetActorLocation` (`self.TARGET`)))
  (set `self.koudousuu` (+ _koudousuu 1))
  (switch `int` (mod _koudousuu 4)
    (:`0`
      (`self.castskill` "敵の攻撃を見極めよう！！" 3.0)
      (set `self.AATimer` 12.0)
      (set `self.eisyounum` 1))
    (:`1`
      (`self.castskill` "矢印が見える攻撃は吹き飛ばされるよ！" 4.0)
      (set `self.AATimer` 12.0)
      (`|SpawnActorFromClass` :`Class` "/Game/BluePrint/gimic/boss1gimic/rakuseki.rakuseki_C" :`SpawnTransform` (`KismetMathLibrary.MakeTransform` _returnvalue) :`CollisionHandlingOverride` "Undefined" :`TransformScaleMethod` "MultiplyWithRoot" :`AoEDamage` 1.0 :`yochoudelay` 7.0 :`Size` 170.0 :`SphereAoE` true :`Knockback` 1300.0 :`penaltyup` false :`Instigator` null))
    (:`2`
      (`self.castskill` "この攻撃は爆心地に近いほどダメージを受けるぞ！離れよう！" 6.0)
      (`|SpawnActorFromClass` "/Game/BluePrint/gimic/boss1gimic/kensasi.kensasi_C" (`KismetMathLibrary.MakeTransform` _returnvalue) "AlwaysSpawn" "MultiplyWithRoot" null 50.0 6.0 null)
      (set `self.AATimer` 12.0))))

(fn `UserConstructionScript`
  (`parent.UserConstructionScript`))