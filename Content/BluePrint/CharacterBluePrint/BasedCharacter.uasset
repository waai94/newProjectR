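; Base combat character for players, AI enemies and bosses, handling HP, status effects, casting and death.
; Goingdamage rolls crits, knockback and resistible effects, then ApplyDamage feeds AnyDamage for defense math, popups and death (exp or boss add count).
; Tick chases the player, advances casts and cooldowns, and rebuilds status flags from CClist, while a looping timer applies DoT/HoT.
; Empty Koudou, Zikkou and Rikou events serve as action, cast-completion and periodic hooks.
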(event `/Game/BluePrint/System/damagekankei.goingdamage`
  (params (damage :type "Float (double-precision)") (isCC :type Boolean) (cc :type "/Game/BluePrint/kouzoutai/joutailist Structure") (causer :type "Actor Object Reference") (knockback :type "Float (double-precision)") (damagetype :type "DamageType Class Reference") (critical :type "Float (double-precision)"))
  (`self.damagefunc` damage isCC cc cc causer causer causer knockback damagetype critical))

(event `dotdamage`
  (bind _cclist (`self.CClist`))
  (`|ExecutionSequence`
    (:`then_0`
      (for _array_element _cclist
        (bind (_crowedcontroll _time _from _strongs) (break `/Game/BluePrint/kouzoutai/joutailist` _array_element))
        (if (`|EnumEquality` _crowedcontroll "NewEnumerator4")
          (`/Game/BluePrint/System/damagekankei.goingdamage` _strongs false (struct) _from 0.0 (select `bool` (< _strongs 0.0) :`false` "/Script/Engine.DamageType" :`true` "/Game/BluePrint/damagetype/heal.heal_C" :!type "DamageType Class Reference")))))
    (:`then_1`
      (for _array_element_2 _cclist
        (bind (_crowedcontroll_2 _time_2 _from_2 _strongs_2) (break `/Game/BluePrint/kouzoutai/joutailist` _array_element_2))
        (if (`|EnumEquality` _crowedcontroll_2 "NewEnumerator5")
          (`/Game/BluePrint/System/damagekankei.goingdamage` _strongs_2 false (struct) _from_2 0.0 "/Game/BluePrint/damagetype/heal.heal_C"))))))

(event `self.ReceiveBeginPlay`
  ;[1 1 1] HP初期設定
  (bind _output_get (set `self.HP` (`self.MAXHP`)))
  (`KismetSystemLibrary.K2_SetTimer` null "dotdamage" 3.0 true)
  (bind _asinstance (cast `/Game/BluePrint/System/instance` (`GameplayStatics.GetGameInstance`)))
  (set `self.nightmaremode` (`/Game/BluePrint/System/instance.isnightmare` _asinstance))
  (bind _asplayer (cast `/Game/BluePrint/CharacterBluePrint/Player` (`GameplayStatics.GetPlayerCharacter` 0)))
  (set `self.player` _asplayer))

(event `self.ReceiveAnyDamage`
  (params (Damage :type "Float (single-precision)") (DamageType :type "DamageType Object Reference") (InstigatedBy :type "Controller Object Reference") (DamageCauser :type "Actor Object Reference"))
  (bind _returnvalue (`GameplayStatics.GetObjectClass` DamageType))
  (bind _returnvalue_2 (`GameplayStatics.GetObjectClass` DamageType))
  (bind _myboss (`self.myboss`))
  (`/Engine/EditorBlueprintResources/StandardMacros.IsValid` DamageCauser
    (:`Is Valid`
      ;[1 1 1] ダメージを与える処理
      (if (== (`|GetArrayItem` (`Actor.Tags` DamageCauser)) (`|GetArrayItem` (`self.Tags`)))
        (if (or (== _returnvalue_2 "/Game/BluePrint/damagetype/heal.heal_C") (== _returnvalue_2 "/Game/BluePrint/damagetype/criticalheal.criticalheal_C"))
          (bind _calceddamage (`self.calcdamage` Damage DamageType :!label _label))
          (bind _returnvalue_3 (`KismetMathLibrary.FTrunc` _calceddamage))
          (set `self.HP` (- (`self.HP`) _returnvalue_3))
          (bind _returnvalue_4 (`|CreateWidget` "/Game/Widget/damagewidget.damagewidget_C" null (`KismetTextLibrary.Conv_IntToText` (`KismetMathLibrary.Abs_Int` _returnvalue_3)) self (select `bool` (< _calceddamage 0.0) :`false` "NewEnumerator0" :`true` "NewEnumerator1" :!type "/Game/BluePrint/rekkyo/damagecolor Enum") (or (== _returnvalue "/Game/BluePrint/damagetype/critical.critical_C") (== _returnvalue "/Game/BluePrint/damagetype/criticalheal.criticalheal_C")) null))
          (`UserWidget.AddToViewport` _returnvalue_4 0)
          (if (<= (`self.HP`) 0.0)
            (`/Engine/EditorBlueprintResources/StandardMacros.DoOnce` false
              (:`Completed`
                (switch `name` (`|GetArrayItem` (`self.Tags`) 1)
                  (:`Default`
                    (set `self.stun` true)
                    (`KismetSystemLibrary.Delay` 1.0)
                    (`self.addexp`)
                    (`self.K2_DestroyActor`))
                  (:`Rikou`
                    (`/Engine/EditorBlueprintResources/StandardMacros.IsValid` _myboss
                      (:`Is Valid`
                        (`self.rikoukazudown` _myboss)
                        (`self.K2_DestroyActor`)))))))))
        (else
          (goto _label))))))

(event `castskill`
  (params (Skillname :type Text) (Casttime :type "Float (double-precision)"))
  (bind _castvar (`self.CastVar`))
  (if (<= (`|GetArrayItem` (`self.skillcooltime`) (`self.eisyounum`)) 0.0)
    ;[1 1 1] 詠唱バーを出現させる。
    (set `self.maxCasttime` Casttime)
    (set `self.Casting` 0.0)
    (set `self.castnow` true)
    (`/Engine/EditorBlueprintResources/StandardMacros.IsValid` _castvar
      (:`Is Valid`
        (`Widget.RemoveFromParent` _castvar))
      (:`Is Not Valid`
        _))
    (bind _returnvalue (`|CreateWidget` "/Game/Widget/castBar.castBar_C" null self Skillname))
    (bind _output_get (set `self.CastVar` _returnvalue))
    (`UserWidget.AddToViewport` _output_get 0)))

(event `self.ReceiveTick`
  (params (DeltaSeconds :type "Float (single-precision)"))
  (bind _maxhp (`self.MAXHP`))
  (bind _aatimer (`self.AATimer`))
  (`|ExecutionSequence`
    (:`then_0`
      (set `CharacterMovementComponent.MaxWalkSpeed` (`KismetMathLibrary.SelectFloat` 0.0 (`KismetMathLibrary.Conv_IntToDouble` (`self.truespeed`)) (or (`self.stun`) (`self.root`))) (`self.CharacterMovement`))
      (set `self.AATimer` (- _aatimer DeltaSeconds))
      (if (and (<= _aatimer 0.0) (<= (`KismetMathLibrary.Vector_Distance` (`self.K2_GetActorLocation`) (`self.K2_GetActorLocation` (`GameplayStatics.GetPlayerCharacter` 0))) (`self.AArange`)))
        (`self.koudou`))
      (`self.castkankei` DeltaSeconds))
    (:`then_1`
      (if (not (`self.IsPlayerControlled`))
        (`|AIMoveTo` self (0.0 0.0 0.0) (`GameplayStatics.GetPlayerCharacter` 0) (- (`self.AArange`) 100.0))))
    (:`then_2`
      (`self.ijousyori`))
    (:`then_3`
      (if (>= (`self.HP`) _maxhp)
        (set `self.HP` _maxhp)))))

(event `skillINTERRUPTED`
  (bind _castvar (`self.CastVar`))
  ;[1 1 1] sukiruchuudan
  (`/Engine/EditorBlueprintResources/StandardMacros.IsValid` _castvar
    (:`Is Valid`
      (`/Game/Widget/castBar.interrupp` _castvar)
      (set `self.castnow` false)
      (`/Game/BluePrint/System/logs.printlogs` "Skill was Interruptted!" "NewEnumerator3"))))

(event `koudou`)

(event `rikoukazudown`
  ;[1 1 1] 履行対象が倒されたら呼び出される。
  (set `self.rikoukazu` (- (`self.rikoukazu`) 1)))

(event `zikkou`)

(event `AutoAttack`
  (bind _atk (`self.ATK`))
  ;[1 1 1] aa
  (`GameplayStatics.ApplyDamage` (`self.TARGET`) (`KismetMathLibrary.Conv_IntToDouble` (+ _atk (`KismetMathLibrary.RandomIntegerInRange` (/ _atk -4) (/ _atk 4)))) null self)
  (set `self.AATimer` (`self.MaxAAtimer`)))

(event `bossintro`
  (bind _returnvalue (`|CreateWidget` "/Game/Widget/bossintro.bossintro_C" null (`KismetTextLibrary.Conv_StringToText` (`KismetStringLibrary.Concat_StrStr` (`KismetTextLibrary.Conv_TextToString` (`self.doublename`)) (`KismetMathLibrary.SelectString` "(Nightmare)" "" (`self.nightmaremode`))))))
  (`UserWidget.AddToViewport` _returnvalue 20))

(event `self.ReceiveActorOnClicked`
  (params (ButtonPressed :type "Key Structure"))
  (message `/Game/BluePrint/System/damagekankei.targetselect` (`GameplayStatics.GetPlayerCharacter` 0) self))

(event `rikou`)

(event `deleteaoe`
  (bind _outactors (`GameplayStatics.GetAllActorsOfClass` "/Game/BluePrint/gimic/AoE.AoE_C"))
  (for _array_element _outactors
    (`self.K2_DestroyActor` _array_element)))

(event `/Game/BluePrint/System/damagekankei.gekiha`
  (`self.castskill` ""))

(fn `addexp`
  (bind _exp (`self.exp`))
  (bind _asplayer (cast `/Game/BluePrint/CharacterBluePrint/Player` (`GameplayStatics.GetPlayerCharacter` 0)))
  (set `/Game/BluePrint/CharacterBluePrint/BasedCharacter.exp` (- _exp (`/Game/BluePrint/CharacterBluePrint/BasedCharacter.exp` _asplayer)) _asplayer)
  (bind _returnvalue (`|CreateWidget` "/Game/Widget/damagewidget.damagewidget_C" null (`KismetTextLibrary.Conv_StringToText` (`KismetStringLibrary.Concat_StrStr` "+" (`KismetStringLibrary.Conv_IntToString` _exp) "exp")) _asplayer "NewEnumerator2" false null))
  (`UserWidget.AddToViewport` _returnvalue 0))

(fn `calcdamage`
  (params (damage :type "Float (double-precision)") (NewParam :type "DamageType Object Reference"))
  (returns (calcedDamage :type "Float (double-precision)"))
  (bind _returnvalue (`GameplayStatics.GetObjectClass` NewParam))
  (return (`KismetMathLibrary.Conv_IntToDouble` (`KismetMathLibrary.FTrunc` (`KismetMathLibrary.FClamp` (`KismetMathLibrary.SelectFloat` (* damage -1.0) (* (`KismetMathLibrary.FClamp` (- damage (`self.DEF`)) 1.0 9999.0) (`KismetMathLibrary.SelectFloat` 0.7 1.0 (and (not (`self.nightmaremode`)) (`self.IsPlayerControlled`)))) (or (== _returnvalue "/Game/BluePrint/damagetype/heal.heal_C") (== _returnvalue "/Game/BluePrint/damagetype/criticalheal.criticalheal_C"))) -9999.0 99999.0)))))

(fn `castkankei`
  (params (B :type "Float (double-precision)"))
  (bind _returnvalue (`GameplayStatics.GetWorldDeltaSeconds`))
  (bind _castvar (`self.CastVar`))
  (bind _casting (`self.Casting`))
  (bind _rikoucharge (`self.rikoucharge`))
  (bind _skillcooltime (`self.skillcooltime`))
  (`|ExecutionSequence`
    (:`then_0`
      (if (`self.castnow`)
        (set `self.Casting` (+ _casting (* B (`KismetMathLibrary.FClamp` (* (`KismetMathLibrary.Conv_IntToDouble` (`self.SPSP`)) 0.02) 1.0 999.0)))))
      (if (>= _casting (`self.maxCasttime`))
        (if (`self.castnow`)
          (set `self.castnow` false)
          (`/Engine/EditorBlueprintResources/StandardMacros.IsValid` _castvar
            (:`Is Valid`
              (`Widget.RemoveFromParent` _castvar)
              (`self.zikkou`))))))
    (:`then_1`
      (if (> _rikoucharge 0.0)
        (set `self.rikoucharge` (- _rikoucharge _returnvalue))
        (else
          (`self.rikou`))))
    (:`then_2`
      (for (_array_element _array_index) _skillcooltime
        (`KismetArrayLibrary.Array_Set` _skillcooltime _array_index (- _array_element _returnvalue))))))

(fn `damagefunc`
  (params (BaseDamage :type "Float (single-precision)") (Condition :type Boolean) (joutailist :type "/Game/BluePrint/kouzoutai/joutailist Structure (by ref)") (InputPin :type "/Game/BluePrint/kouzoutai/joutailist Structure") (self2 :type "Actor Object Reference") (self3 :type "Actor Object Reference") (DamageCauser :type "Actor Object Reference") (B :type "Float (double-precision)") (damagetype :type "DamageType Class Reference") (ctiritcal :type "Float (double-precision)"))
  (locals (equalcc :type Boolean) (damaged :type "Float (double-precision)" :default 1.0) (onazitag :type Boolean) (notice :type Text) (criticalhit :type Boolean) (muteki :type Boolean))
  (bind _crowedcontroll (break `/Game/BluePrint/kouzoutai/joutailist` InputPin))
  (bind (_crowedcontroll_2 _time _from _strongs _koukanamae _canstack _membervar_20 _setumei _isally) (break `/Game/BluePrint/kouzoutai/joutailist` InputPin))
  (bind _returnvalue (== damagetype "/Game/BluePrint/damagetype/heal.heal_C"))
  (bind _cclist (`self.CClist`))
  (bind _charactermovement (`self.CharacterMovement`))
  (bind _damaged (`local.damaged`))
  (bind _criticalhit (`local.criticalhit`))
  (bind (_returnvalue_roll _returnvalue_pitch _returnvalue_yaw) (`KismetMathLibrary.BreakRotator` (`KismetMathLibrary.FindLookAtRotation` (`self.K2_GetActorLocation` self2) (`self.K2_GetActorLocation`))))
  (bind _returnvalue_2 (== (`|GetArrayItem` (`Actor.Tags` self3)) (`|GetArrayItem` (`self.Tags`))))
  (bind (_crowedcontroll_3 _time_2) (break `/Game/BluePrint/kouzoutai/joutailist` (`|GetArrayItem` (`self.CCtaisei`) (select `/Game/BluePrint/rekkyo/joutaiijou` _crowedcontroll :`NewEnumerator1` 1 :`NewEnumerator2` 2 :`NewEnumerator3` 3 :`NewEnumerator4` 4 :`NewEnumerator5` 5 :`NewEnumerator6` 6 :`NewEnumerator7` 7 :`NewEnumerator8` 8))))
  (for _array_element (`self.CClist`)
    (if (`|EnumEquality` (`.CrowedControll_2_37B9E4024FA5C4692A534DB1AAEB5F06` (break `/Game/BluePrint/kouzoutai/joutailist` _array_element)) "NewEnumerator7")
      (set `local.muteki` true)))
  (set `local.criticalhit` (>= ctiritcal (`KismetMathLibrary.RandomFloatInRange` 0.0 100.0)))
  (for _array_element_2 (`self.CClist`)
    (bind (_crowedcontroll_4 _time_3 _from_2 _strongs_2) (break `/Game/BluePrint/kouzoutai/joutailist` _array_element_2))
    (if (`|EnumEquality` _crowedcontroll_4 "NewEnumerator6")
      (set `local.damaged` (+ _damaged _strongs_2))))
  (if (not (`local.muteki`))
    (`GameplayStatics.ApplyDamage` self (`KismetMathLibrary.SelectFloat` BaseDamage (* BaseDamage _damaged (`KismetMathLibrary.SelectFloat` 1.6 1.0 _criticalhit)) _returnvalue) null DamageCauser (select `bool` _criticalhit :`false` damagetype :`true` (select `bool` _returnvalue :`false` "/Game/BluePrint/damagetype/critical.critical_C" :`true` "/Game/BluePrint/damagetype/criticalheal.criticalheal_C" :!type "DamageType Class Reference")))
    ;[1 1 1] goingdamage
    (set `local.onazitag` _returnvalue_2)
    (if (not _returnvalue_2)
      (`/Engine/EditorBlueprintResources/StandardMacros.IsValid` _charactermovement
        (:`Is Valid`
          (`CharacterMovementComponent.AddImpulse` _charactermovement (* (`KismetMathLibrary.Normal` (`KismetMathLibrary.GetForwardVector` (`KismetMathLibrary.MakeRotator` _returnvalue_roll 1.0 _returnvalue_yaw))) B (1.0 1.0 10.0)) true))
        (:`Is Not Valid`
          _)))
    (if Condition
      (if (>= (`KismetMathLibrary.RandomFloatInRange` 0.0 99.0) _time_2)
        (if (and (`local.onazitag`) (or (`|EnumEquality` _crowedcontroll_2 "NewEnumerator5") _isally))
          (for (_array_element_3 _array_index) _cclist :!label _label
            (if (== (`.koukanamae_16_952C240D43E33C81C60FD6A362E0B7EA` (break `/Game/BluePrint/kouzoutai/joutailist` _array_element_3)) _koukanamae)
              (set `local.equalcc` true)
              (break)))
          (if (and (`local.equalcc`) (not _canstack))
            (`KismetArrayLibrary.Array_Set` _cclist _array_index InputPin)
            (else
              (`KismetArrayLibrary.Array_Add` (`self.CClist`) InputPin)))
          (bind _returnvalue_3 (`|CreateWidget` "/Game/Widget/damagewidget.damagewidget_C" null _koukanamae self "NewEnumerator2" false (`.MemberVar_20_21_E07DE1CD47371F18A70DA6BFCF052EA8` (break `/Game/BluePrint/kouzoutai/joutailist` InputPin))))
          (`UserWidget.AddToViewport` _returnvalue_3 0)
          (switch `/Game/BluePrint/rekkyo/joutaiijou` (`.CrowedControll_2_37B9E4024FA5C4692A534DB1AAEB5F06` (break `/Game/BluePrint/kouzoutai/joutailist` joutailist))
            (:`NewEnumerator0`
              _)
            (:`NewEnumerator2`
              _))
          (`self.skillINTERRUPTED`)
          (elif (not (`local.onazitag`))
            (goto _label)))
        (else
          (set `local.notice` (`KismetTextLibrary.Conv_StringToText` (`KismetStringLibrary.Concat_StrStr` (`|GetEnumeratorNameAsString` _crowedcontroll) (`KismetMathLibrary.SelectString` "(Nope)" "(Resist)" (== _time_2 100.0))))))))))

(fn `ijousyori`
  (locals (attackbuff :type "Float (double-precision)" :default 1.0) (nowcc :type "/Game/BluePrint/kouzoutai/joutailist Structure"))
  (bind _cclist (`self.CClist`))
  (set `self.truespeed` (`self.SPD`))
  (set `self.slow` false)
  (set `self.fear` false)
  (set `self.root` false)
  (set `self.stun` false)
  (for (_array_element _array_index) (`self.CClist`)
    (set `local.nowcc` _array_element)
    (`|ExecutionSequence`
      (:`then_0`
        (bind (_crowedcontroll _time _from _strongs _koukanamae _canstack _membervar_20 _setumei) (break `/Game/BluePrint/kouzoutai/joutailist` _array_element))
        (switch `/Game/BluePrint/rekkyo/joutaiijou` _crowedcontroll
          (:`NewEnumerator0`
            (set `self.stun` true))
          (:`NewEnumerator1`
            (set `self.root` true))
          (:`NewEnumerator2`
            (set `self.fear` true))
          (:`NewEnumerator3`
            (set `self.slow` true))
          (:`NewEnumerator8`
            (set `self.truespeed` (`KismetMathLibrary.FTrunc` (* (`KismetMathLibrary.Conv_IntToDouble` (`self.truespeed`)) _strongs))))
          (:`NewEnumerator9`
            (set `local.attackbuff` (* (`local.attackbuff`) (`.Strongs_13_F61493A945C00D04E51AE08D8E9349BB` (break `/Game/BluePrint/kouzoutai/joutailist` (`local.nowcc`))))))))
      (:`then_2`
        (`KismetArrayLibrary.Array_Set` _cclist _array_index (make `/Game/BluePrint/kouzoutai/joutailist` _crowedcontroll (- _time (`GameplayStatics.GetWorldDeltaSeconds`)) _from _strongs _koukanamae _canstack _membervar_20 _setumei))
        (if (<= _time 0.0)
          (bind _returnvalue (`|CreateWidget` "/Game/Widget/damagewidget.damagewidget_C" null (`KismetTextLibrary.Conv_StringToText` (`KismetStringLibrary.Concat_StrStr` "-" (`KismetTextLibrary.Conv_TextToString` _koukanamae))) self "NewEnumerator2" false _membervar_20))
          (`KismetArrayLibrary.Array_Remove` _cclist _array_index)
          (`UserWidget.AddToViewport` _returnvalue 0)))))
  (set `self.calcatk` (`KismetMathLibrary.FTrunc` (* (`self.ATK`) (`local.attackbuff`)))))

(fn `moveto`)

(fn `OnRep_exp`
  (if (<= (`self.exp`) 0)
    (`/Game/BluePrint/System/damagekankei.levelchange`)))

(fn `UserConstructionScript`)