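; Sorcerer (jujutushi) character Blueprint that attacks player character 0 with cast fire spells, building on a parent class.
; Koudou counts actions, casting "ファイア" normally and "オメガファイア" every fourth time, and records the chosen spell in Eisyounum.
; Zikkou dispatches on that index: Zangeki spawns a Firemahou actor given the target, while Kuromahou drops a delayed spherical AoE at the target's location.
; Both spells scale damage from ATK.
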(event `self.zikkou`
  (switch `int` (`self.eisyounum`)
    (:`0`
      (`self.zangeki`))
    (:`1`
      (`self.kuromahou`))))

(event `kuromahou`
  (`|SpawnActorFromClass` :`Class` "/Game/BluePrint/gimic/AoE.AoE_C" :`SpawnTransform` (`KismetMathLibrary.MakeTransform` (`self.K2_GetActorLocation` (`self.TARGET`))) :`CollisionHandlingOverride` "AlwaysSpawn" :`TransformScaleMethod` "MultiplyWithRoot" :`AoEDamage` (`KismetMathLibrary.Conv_IntToDouble` (* (`self.ATK`) 6)) :`delayed` 1.0 :`Size` 40.0 :`SphereAoE` true :`Instigator` null))

(event `self.ReceiveBeginPlay`
  (`parent.ReceiveBeginPlay`)
  (set `self.TARGET` (`GameplayStatics.GetPlayerCharacter` 0)))

(event `zangeki`
  (`|SpawnActorFromClass` "/Game/BluePrint/firemahou.firemahou_C" (`self.GetTransform`) "AlwaysSpawn" "MultiplyWithRoot" null (* (`KismetMathLibrary.Conv_IntToDouble` (`self.ATK`)) 1.25) (`self.TARGET`) 0.0 null))

(event `self.koudou`
  (bind _koudousuu (`self.koudousuu`))
  (set `self.koudousuu` (+ _koudousuu 1))
  (if (== (mod _koudousuu 4) 0)
    (`self.castskill` "オメガファイア" 1.0)
    (set `self.AATimer` 4.0)
    (set `self.eisyounum` 1)
    (else
      (`self.castskill` "ファイア" 2.0)
      (set `self.AATimer` 4.0)
      (set `self.eisyounum` 0))))

(fn `UserConstructionScript`
  (`parent.UserConstructionScript`))