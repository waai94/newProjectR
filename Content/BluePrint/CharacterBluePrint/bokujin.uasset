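; Enemy caster Blueprint "bokujin" that targets player 0 and attacks with cast-time skills.
; Koudou starts a named cast, setting AATimer and Eisyounum; Zikkou switches on that number to spawn the spell.
; Kuromahou drops a delayed spherical Rakuseki AoE at the player's location; Zangeki spawns a targeted Firemahou scaled from ATK.
; Only the AoE cast is wired into Koudou; the every-fourth-action rotation with Fire is disconnected.
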(event `self.zikkou`
  (switch `int` (`self.eisyounum`)
    (:`0`
      (`self.zangeki`))
    (:`1`
      (`self.kuromahou`))))

(event `kuromahou`
  (`|SpawnActorFromClass` :`Class` "/Game/BluePrint/gimic/boss1gimic/rakuseki.rakuseki_C" :`SpawnTransform` (`KismetMathLibrary.MakeTransform` (`self.K2_GetActorLocation` (`self.TARGET`))) :`CollisionHandlingOverride` "AlwaysSpawn" :`TransformScaleMethod` "MultiplyWithRoot" :`AoEDamage` 1.0 :`yochoudelay` 8.0 :`Size` 20.0 :`SphereAoE` true :`Instigator` null))

(event `self.ReceiveBeginPlay`
  (`parent.ReceiveBeginPlay`)
  (set `self.TARGET` (`GameplayStatics.GetPlayerCharacter` 0)))

(event `zangeki`
  (`|SpawnActorFromClass` "/Game/BluePrint/firemahou.firemahou_C" (`self.GetTransform`) "AlwaysSpawn" "MultiplyWithRoot" null (* (`KismetMathLibrary.Conv_IntToDouble` (`self.ATK`)) 1.25) (`self.TARGET`) 0.0 null))

(event `self.koudou`
  (`self.castskill` "赤い範囲をよけろ！" 3.0)
  (set `self.AATimer` 12.0)
  (set `self.eisyounum` 1))

(fn `UserConstructionScript`
  (`parent.UserConstructionScript`))