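; Enemy template Blueprint that gives an example of randomized enemy combat behaviour.
; The Koudou event randomly picks one of three actions: a printed auto-attack, a skill cast, or a longer cast that interrupts itself partway through.
; Each action sets AATimer, and skills go through Castskill and SkillINTERRUPTED.
; A counter-based action cycle is present but left disconnected.
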(event `self.ReceiveBeginPlay`
  (`parent.ReceiveBeginPlay`))

(event `self.koudou`
  ;[1 1 1] ランダム行動のプログラム例です。
  (switch `int` (`KismetMathLibrary.RandomIntegerInRange` 0 2)
    (:`0`
      (`KismetSystemLibrary.PrintString` "オートアタック")
      (set `self.AATimer` 2.0))
    (:`1`
      (`self.castskill` "敵のスキル" 3.0)
      (set `self.AATimer` 6.0))
    (:`2`
      (set `self.AATimer` 6.0)
      (`self.castskill` "敵のスキル" 6.0)
      (`KismetSystemLibrary.Delay` 3.0)
      (`self.skillINTERRUPTED`))))

(fn `UserConstructionScript`
  (`parent.UserConstructionScript`))