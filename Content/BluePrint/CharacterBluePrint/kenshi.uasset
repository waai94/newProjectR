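; Kenshi (swordsman) combat character Blueprint that targets the player and builds on a parent class's action and casting system.
; Koudou counts actions, auto-attacking except on every fourth, when it starts casting the 斬撃 (slash) skill.
; Zikkou fires Kyouzangeki, sending ATK-scaled damage with a timed crowd-control effect through GoingdamageMessage.
; The plain zangeki ApplyDamage event is referenced only by disconnected nodes.
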(event `kyouzangeki`
  (message `/Game/BluePrint/System/damagekankei.goingdamage` (`self.TARGET`) (* (`KismetMathLibrary.Conv_IntToDouble` (`self.ATK`)) 1.25) true (make `/Game/BluePrint/kouzoutai/joutailist` "NewEnumerator0" 3.0 self 0.0 "" false "/Game/Texture/icons/debuff/vitup.vitup" "" false false 0.0 "" "" null) null 0.0 null 0.0))

(event `self.zikkou`
  (`self.kyouzangeki`))

(event `zangeki`
  (`GameplayStatics.ApplyDamage` (`self.TARGET`) (* (`KismetMathLibrary.Conv_IntToDouble` (`self.ATK`)) 1.25)))

(event `self.ReceiveBeginPlay`
  (`parent.ReceiveBeginPlay`)
  (set `self.TARGET` (`GameplayStatics.GetPlayerCharacter` 0)))

(event `self.koudou`
  (bind _koudousuu (`self.koudousuu`))
  (set `self.koudousuu` (+ _koudousuu 1))
  (if (== (mod _koudousuu 4) 0)
    (`self.castskill` "斬撃" 2.0)
    (set `self.AATimer` 4.0)
    (set `self.eisyounum` 0)
    (else
      (`self.AutoAttack`))))

(fn `UserConstructionScript`
  (`parent.UserConstructionScript`))