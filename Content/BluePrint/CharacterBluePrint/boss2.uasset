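; Time-themed boss that chains timed casts of clock AoEs, eruptions, knockback and delayed time-stop/rewind debuffs on the player.
; BeginPlay runs only the Kouhannightmare sequence; the longer opening rotation is disconnected.
; Helpers spawn telegraphed attacks, then reverse or restart them with Niagara clock and line cues, using shuffled or random picks.
; Changekeitai, also disconnected, stages a giant chained prison cast ending in game over or interruption back to Kouhannightmare.
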(event `self.ReceiveBeginPlay`
  (`parent.ReceiveBeginPlay`)
  (set `self.firstpos` (`self.K2_GetActorLocation`))
  (`self.kouhannightmare`))

(event `kouhannightmare`
  (`self.castskill` "定められ士運命" 3.0)
  (`KismetSystemLibrary.Delay` 3.0)
  (`self.applytimejudge` 20.0)
  (`KismetSystemLibrary.Delay` 7.0)
  (`|SpawnActorFromClass` :`Class` "/Game/BluePrint/gimic/boss2gimic/timehuttobashi.timehuttobashi_C" :`SpawnTransform` (`KismetMathLibrary.MakeTransform` (+ (`self.firstpos`) (0.0 0.0 0.0))) :`CollisionHandlingOverride` "AlwaysSpawn" :`TransformScaleMethod` "MultiplyWithRoot" :`AoEDamage` 100.0 :`yochoudelay` 15.0 :`Size` 999.0 :`SphereAoE` true :`Knockback` 2000.0 :`penaltyup` false :`Instigator` null)
  (`KismetSystemLibrary.Delay` 7.0)
  (`self.circletimeeraption` false)
  (`KismetSystemLibrary.Delay` 20.0)
  (`self.castskill` "定めし運命：時間逆行" 4.0)
  (`KismetSystemLibrary.Delay` 4.0)
  (`self.backdebuff` 15.0)
  (`KismetSystemLibrary.Delay` 4.0)
  (`self.timerattackgo` (0.0 0.0 0.0) 5 0.4 false true))

(event `changekeitai`
  (`self.K2_SetActorLocation` (2700.0 0.0 0.0))
  (`self.SetActorScale3D` (20.0 20.0 20.0))
  (`KismetSystemLibrary.Delay` 3.0)
  (for _index (range 3)
    (`|SpawnActorFromClass` "/Game/BluePrint/gimic/boss2gimic/kusari.kusari_C" (`KismetMathLibrary.MakeTransform` (0.0 0.0 0.0) (select `int` _index :`0` (struct :`Pitch` -45.0) :`1` (struct :`Pitch` -64.233758 :`Yaw` -80.382428 :`Roll` 167.539129) :`2` (struct :`Pitch` -4.702439 :`Yaw` 149.652662 :`Roll` -40.827678) :!type "Rotator Structure")) "Undefined" "MultiplyWithRoot" null null))
  (`|SpawnActorFromClass` "/Game/BluePrint/CharacterBluePrint/tokinorougoku.tokinorougoku_C" (`KismetMathLibrary.MakeTransform` (0.0 0.0 120.0)) "AlwaysSpawn" "MultiplyWithRoot" null self null)
  (`KismetSystemLibrary.K2_SetTimer` null "rikoutimeerap" 3.0 true)
  (set `self.rikoucharge` 45.0)
  (`self.castskill` "判決：終身刑" 45.0)
  (goto _label :!via `Reset`))

(event `self.ReceiveTick`
  (params (DeltaSeconds :type "Float (single-precision)"))
  (`parent.ReceiveTick` DeltaSeconds)
  (set `self.time` (+ (`self.time`) DeltaSeconds)))

(event `timerattackfirst`
  (params (forwardvector :type "Vector Structure") (loop :type Integer) (randomtime :type "Float (double-precision)") (toplayer :type Boolean))
  (`self.castskill` "クロックバースト" 6.0)
  (for _ (range (+ loop 1))
    (`self.maketimerAoE` forwardvector 0.6 1.0 randomtime toplayer 7.0)
    (`KismetSystemLibrary.Delay` 7.5)
    (`self.castskill` "アンチクロックワイズ" 5.0)
    (`self.reverse` 0 5.0)))

(event `self.rikou`
  (`/Engine/EditorBlueprintResources/StandardMacros.DoOnce` false :!label _label
    (:`Completed`
      (`KismetSystemLibrary.K2_ClearTimer` null "rikoutimeerap")
      (if (<= (`self.rikoucharge`) 0.0)
        (message `/Game/BluePrint/System/damagekankei.goingdamage` (`GameplayStatics.GetPlayerCharacter` 0) 0.0 true (make `/Game/BluePrint/kouzoutai/joutailist` "NewEnumerator12" 999.0 null 0.0 "時の監獄" false "/Game/Texture/icons/debuff/vitup.vitup" "時の牢獄にとらえられた状態。" false false 0.0 "" "" null) self 0.0 null 0.0)
        (`KismetSystemLibrary.Delay` 2.0)
        (`/Game/BluePrint/System/noticeui.noticewidgetcreate` "閉じ込められてしまった…")
        (`KismetSystemLibrary.Delay` 4.0)
        (`GameplayStatics.SetGamePaused` true)
        (bind _returnvalue (`|CreateWidget` "/Game/Widget/gameover.gameover_C"))
        (`UserWidget.AddToViewport` _returnvalue 0)
        (else
          (bind _outactors (`GameplayStatics.GetAllActorsOfClass` "/Game/BluePrint/gimic/boss2gimic/kusari.kusari_C"))
          (`self.skillINTERRUPTED`)
          (for _array_element _outactors
            (`self.K2_DestroyActor` _array_element))
          (`self.kouhannightmare`))))))

(event `self.rikoukazudown`
  (`self.rikou`))

(event `addtoplayerCC`
  (`self.castskill` "時空掌握" 4.0)
  (`|SpawnActorFromClass` "/Game/BluePrint/gimic/playernerai.playernerai_C" (`KismetMathLibrary.MakeTransform` (0.0 0.0 0.0)) "Undefined" "MultiplyWithRoot" null (`GameplayStatics.GetPlayerCharacter` 0) 4.0 null)
  (`KismetSystemLibrary.Delay` 4.0)
  (message `/Game/BluePrint/System/damagekankei.goingdamage` (`GameplayStatics.GetPlayerCharacter` 0) 150.0 true (make `/Game/BluePrint/kouzoutai/joutailist` "NewEnumerator11" 14.0 self 120.0 "加速度爆弾" false "/Game/Texture/icons/debuff/stun.stun" "効果時間が終了時、動いているとダメージを受ける。" false false 3.0 "時の拘束" "時空に拘束された状態。" "/Game/Texture/icons/debuff/stun.stun") self 0.0 null 0.0))

(event `rikoutimeattack`
  (params (forwardvector :type "Vector Structure") (loop :type Integer) (randomtime :type "Float (double-precision)") (toplayer :type Boolean) (randomtoplayer :type Boolean) (speed :type "Float (double-precision)" :default 1.0) (stoptime :type "Float (double-precision)"))
  (`self.castskill` "" 6.0)
  (for _ (range (+ loop 1))
    (`self.maketimerAoE` (0.0 0.0 0.0) stoptime speed randomtime (select `bool` randomtoplayer :`false` toplayer :`true` (`KismetMathLibrary.RandomBool`)) 7.0)
    (`KismetSystemLibrary.Delay` 7.5)
    (if (< stoptime 1.0)
      (`self.castskill` "再始動" 5.0)
      (`self.reverse` 1 5.0 (/ loop 2)))))

(event `timerattackgo`
  (params (forwardvector :type "Vector Structure") (loop :type Integer) (randomtime :type "Float (double-precision)") (toplayer :type Boolean) (randomtoplayer :type Boolean) (speed :type "Float (double-precision)" :default 1.0) (stoptime :type "Float (double-precision)"))
  (`self.castskill` "クロックバースト" 6.0)
  (for _ (range (+ loop 1))
    (`self.maketimerAoE` forwardvector stoptime speed randomtime (select `bool` randomtoplayer :`false` toplayer :`true` (`KismetMathLibrary.RandomBool`)) 7.0)
    (`KismetSystemLibrary.Delay` 7.5)
    (if (< stoptime 1.0)
      (`self.castskill` "再始動" 5.0)
      (`self.reverse` 1 5.0 (/ loop 2)))))

(event `applytimejudge`
  (params (Time :type "Float (double-precision)"))
  (message `/Game/BluePrint/System/damagekankei.goingdamage` (`GameplayStatics.GetPlayerCharacter` 0) 0.0 true (make `/Game/BluePrint/kouzoutai/joutailist` "NewEnumerator12" Time self 0.0 "定めし運命：時間停止" false "/Game/Texture/icons/debuff/stun.stun" "効果終了後に時間停止を受ける。" false true 8.0 "運命：時間停止" "時間が止められた" "/Game/Texture/icons/debuff/stun.stun") self 0.0 null 0.0))

(event `backdebuff`
  (params (Time :type "Float (double-precision)"))
  (bind _returnvalue (`GameplayStatics.GetPlayerCharacter` 0))
  (message `/Game/BluePrint/System/damagekankei.goingdamage` _returnvalue 0.0 true (make `/Game/BluePrint/kouzoutai/joutailist` "NewEnumerator13" Time self 0.0 "定めし運命：時間逆行" false "/Game/Texture/icons/debuff/stun.stun" "効果終了後に時間がさかのぼる。" false false 8.0 "運命：時間停止" "時間が止められた" "/Game/Texture/icons/debuff/stun.stun") self 0.0 null 0.0)
  (message `/Game/BluePrint/System/damagekankei.reversetime` _returnvalue Time)
  (`/Game/BluePrint/System/logs.printlogs` "dawdwa"))

(event `circletimeeraption`
  (params (mannnaka :type Boolean))
  (bind _firstpos (`self.firstpos`))
  (`self.castskill` "タイムエラプション" 3.0)
  (`KismetSystemLibrary.Delay` 3.0)
  (for _index (range 8)
    (`|SpawnActorFromClass` :`Class` "/Game/BluePrint/gimic/boss2gimic/timerap.timerap_C" :`SpawnTransform` (`KismetMathLibrary.MakeTransform` (+ _firstpos (* (`KismetMathLibrary.Conv_RotatorToVector` (`KismetMathLibrary.MakeRotator` 0.0 0.0 (`KismetMathLibrary.Conv_IntToDouble` (* _index 45)))) 1500))) :`CollisionHandlingOverride` "AlwaysSpawn" :`TransformScaleMethod` "MultiplyWithRoot" :`AoEDamage` 200.0 :`Size` 20.0 :`SphereAoE` true :`Instigator` null))
  (if mannnaka
    (`|SpawnActorFromClass` :`Class` "/Game/BluePrint/gimic/boss2gimic/timerap.timerap_C" :`SpawnTransform` (`KismetMathLibrary.Conv_VectorToTransform` _firstpos) :`CollisionHandlingOverride` "AlwaysSpawn" :`TransformScaleMethod` "MultiplyWithRoot" :`AoEDamage` 200.0 :`Size` 20.0 :`SphereAoE` true :`Instigator` null)))

(event `circletimeattack`
  (`self.castskill` "ビームオブタイム" 6.0)
  (`self.setcircle`))

(event `timeeraption`
  ;[1 1 1] 所要時間３４秒
  (`KismetArrayLibrary.Array_Clear` (`self.atarierap`))
  (`self.castskill` "タイムバースト" 6.0)
  (`self.createtimeera@tion` 0 true)
  (`KismetSystemLibrary.Delay` 8.0)
  (`self.castskill` "タイムバースト" 6.0)
  (`self.createtimeera@tion` 1 true)
  (`KismetSystemLibrary.Delay` 8.0)
  (`self.castskill` "タイムバースト" 6.0)
  (`self.createtimeera@tion` 2)
  (`KismetSystemLibrary.Delay` 8.0)
  (`self.castskill` "アンチクロックワイズ" 4.0)
  (set `self.seikai` (`KismetMathLibrary.RandomIntegerInRange` 0 2))
  (`self.modoru`)
  (`KismetSystemLibrary.Delay` 4.0)
  (`self.castskill` "タイムバースト" 6.0)
  (`self.createtimeera@tion` (`self.seikai`) false true))

(fn `createsen`
  (params (target :type "Vector Structure"))
  (bind _returnvalue (`NiagaraFunctionLibrary.SpawnSystemAtLocation` "/Game/effect/tekinokougeki/line.line" (`self.K2_GetActorLocation`)))
  (`FXSystemComponent.SetVectorParameter` _returnvalue "vector" target))

(fn `createtimeera@tion`
  (params (kaisuu :type Integer) (afterdestroy :type Boolean) (modrigo :type Boolean))
  (bind _returnvalue (`self.K2_GetActorLocation`))
  (`KismetArrayLibrary.Array_Add` (`self.atarierap`) (`KismetMathLibrary.RandomIntegerInRange` 0 3))
  (for _index (range 4)
    (`|SpawnActorFromClass` :`Class` "/Game/BluePrint/gimic/boss2gimic/eraption.eraption_C" :`SpawnTransform` (`KismetMathLibrary.MakeTransform` (+ _returnvalue (* (`KismetMathLibrary.GetForwardVector` (`KismetMathLibrary.MakeRotator` 0.0 0.0 (+ (`KismetMathLibrary.Conv_IntToDouble` (* _index 90)) 45.0))) 1500))) :`CollisionHandlingOverride` "Undefined" :`TransformScaleMethod` "MultiplyWithRoot" :`afterdestroy` afterdestroy :`AoEDamage` 300.0 :`yochoudelay` (`KismetMathLibrary.SelectFloat` 1.0 6.0 modrigo) :`Size` 47.0 :`SphereAoE` true :`ringdistance` (`KismetMathLibrary.SelectFloat` 20.0 0.0 (== _index (`|GetArrayItem` (`self.atarierap`) kaisuu))) :`jobantaiki` (`KismetMathLibrary.SelectFloat` 5.0 0.0 modrigo) :`Instigator` null))
  (`|SpawnActorFromClass` :`Class` "/Game/BluePrint/gimic/boss2gimic/eraption.eraption_C" :`SpawnTransform` (`KismetMathLibrary.Conv_VectorToTransform` _returnvalue) :`CollisionHandlingOverride` "AlwaysSpawn" :`TransformScaleMethod` "MultiplyWithRoot" :`afterdestroy` afterdestroy :`AoEDamage` 300.0 :`yochoudelay` 6.0 :`Size` 26.0 :`SphereAoE` true :`Instigator` null))

(fn `maketimerAoE`
  (params (A :type "Vector Structure") (stoptime :type "Float (double-precision)") (timespeed :type "Float (double-precision)" :default 1.0) (randomtime :type "Float (double-precision)") (toplayer :type Boolean) (timesize1 :type "Float (double-precision)" :default 10.0))
  (locals (setpoint :type "Vector Structure") (rotate :type "Rotator Structure" :default (struct)) (timesize :type "Float (double-precision)"))
  (bind _returnvalue (== A (0.0 0.0 0.0)))
  (bind _timesize (`local.timesize`))
  (bind _yaw (.yaw (`local.rotate`)))
  (set `local.timesize` timesize1)
  (set `local.rotate` (`KismetMathLibrary.RandomRotator` false))
  (bind _output_get (set `local.setpoint` (+ (`self.K2_GetActorLocation`) (* (`KismetMathLibrary.SelectVector` (`KismetMathLibrary.GetForwardVector` (`KismetMathLibrary.MakeRotator` 0.0 0.0 _yaw)) A _returnvalue) 2000))))
  (`|SpawnActorFromClass` "/Game/BluePrint/gimic/boss2gimic/timeaoe.timeaoe_C" (`KismetMathLibrary.MakeTransform` _output_get (`KismetMathLibrary.MakeRotator` 0.0 0.0 (.yaw (`KismetMathLibrary.SelectRotator` (`KismetMathLibrary.FindLookAtRotation` (`local.setpoint`) (`self.K2_GetActorLocation` (`GameplayStatics.GetPlayerCharacter` 0))) (`KismetMathLibrary.MakeRotator` 0.0 0.0 (`KismetMathLibrary.SelectFloat` (+ _yaw 180.0) (+ (.yaw (`KismetMathLibrary.Conv_VectorToRotator` A)) 180.0) _returnvalue)) toplayer))) (`KismetMathLibrary.MakeVector` _timesize _timesize _timesize)) "AlwaysSpawn" "MultiplyWithRoot" null timespeed (+ stoptime randomtime) 160.0 6.0 0.0 1.0 false 0.0 0.0 0.0 false (`|MakeArray` (make `/Game/BluePrint/kouzoutai/joutailist` "NewEnumerator0" 3.0 self 1.0 "時の拘束" false "/Game/Texture/icons/debuff/vitup.vitup" "時空に拘束されている状態。" false false 0.0 "" "" null)) null))

(fn `modoru`
  (bind _seikai (`self.seikai`))
  (bind _outactors (`GameplayStatics.GetAllActorsOfClass` "/Game/BluePrint/gimic/boss2gimic/eraption.eraption_C"))
  (for _array_element _outactors
    (bind _returnvalue (`self.K2_GetActorLocation` _array_element))
    (bind _returnvalue_2 (`NiagaraFunctionLibrary.SpawnSystemAtLocation` "/Game/effect/tekinokougeki/clock.clock" (+ _returnvalue (0.0 0.0 300.0)) (struct :`Yaw` -45.0)))
    (`FXSystemComponent.SetFloatParameter` _returnvalue_2 "float" (* 1.0 (select `int` _seikai :`0` 9.0 :`1` 3.0 :`2` 1.0)))
    (`self.createsen` _returnvalue)
    (`/Game/BluePrint/System/noticeui.noticewidgetcreate` (select `int` _seikai :`0` "時がかなり巻き戻る！" :`1` "時が更に巻き戻る！" :`2` "時が巻き戻る！" :!type "Text"))))

(fn `reverse`
  (params (whatpt :type Integer) (time :type "Float (double-precision)") (kousu :type Integer))
  (locals (aoe :type "Array of /Game/BluePrint/gimic/boss2gimic/timeaoe Object Reference") (cll :type "Array of Actor Object Reference"))
  (bind _aoe (`local.aoe`))
  (bind _cll (`local.cll`))
  (`|ExecutionSequence`
    (:`then_0`
      (bind _outactors (`GameplayStatics.GetAllActorsOfClass` "/Game/BluePrint/gimic/boss2gimic/timeaoe.timeaoe_C"))
      (bind _output_get (set `local.aoe` _outactors))
      (`KismetArrayLibrary.Array_Shuffle` _output_get)
      (switch `int` whatpt
        (:`0`
          (for _array_element (`local.aoe`)
            (`KismetSystemLibrary.K2_SetTimer` _array_element "reverse" time)
            (`KismetArrayLibrary.Array_Add` _cll _array_element)
            (`NiagaraFunctionLibrary.SpawnSystemAtLocation` "/Game/effect/tekinokougeki/clock.clock" (+ (`SceneComponent.K2_GetComponentLocation` (`/Game/BluePrint/gimic/boss2gimic/timeaoe.kougeki` _array_element)) (0.0 0.0 1000.0)) (struct :`Yaw` -45.0))))
        (:`1`
          (for _index (range (+ kousu 1))
            (bind _output (`|GetArrayItem` _aoe _index))
            (`KismetSystemLibrary.K2_SetTimer` _output "reverse" time)
            (`KismetArrayLibrary.Array_Add` _cll _output)
            (`NiagaraFunctionLibrary.SpawnSystemAtLocation` "/Game/effect/tekinokougeki/clock.clock" (+ (`SceneComponent.K2_GetComponentLocation` (`/Game/BluePrint/gimic/boss2gimic/timeaoe.kougeki` _output)) (0.0 0.0 1000.0)) (struct :`Yaw` -45.0)))
          (for _index_2 (range _index (+ (`KismetArrayLibrary.Array_Length` _aoe) 1))
            (bind _output_2 (`|GetArrayItem` _aoe _index_2))
            (`/Engine/EditorBlueprintResources/StandardMacros.IsValid` _output_2
              (:`Is Valid`
                (`/Game/BluePrint/System/logs.printlogs` "goagain")
                (`KismetSystemLibrary.K2_SetTimer` _output_2 "again" time)
                (`KismetArrayLibrary.Array_Add` (`local.cll`) _output_2)
                (bind _returnvalue (`NiagaraFunctionLibrary.SpawnSystemAtLocation` "/Game/effect/tekinokougeki/clock.clock" (+ (`SceneComponent.K2_GetComponentLocation` (`/Game/BluePrint/gimic/boss2gimic/timeaoe.kougeki` _output_2)) (0.0 0.0 1000.0)) (struct :`Yaw` 135.0)))
                (`FXSystemComponent.SetFloatParameter` _returnvalue "float" 1.0)))))))
    (:`then_1`
      (for _array_element_2 (`local.cll`)
        (bind _astimeaoe (cast `/Game/BluePrint/gimic/boss2gimic/timeaoe` _array_element_2))
        (bind _returnvalue_2 (`NiagaraFunctionLibrary.SpawnSystemAtLocation` "/Game/effect/tekinokougeki/line.line" (`self.K2_GetActorLocation`)))
        (`FXSystemComponent.SetVectorParameter` _returnvalue_2 "vector" (`SceneComponent.K2_GetComponentLocation` (`/Game/BluePrint/gimic/boss2gimic/timeaoe.kougeki` _astimeaoe)))))))

(fn `rikoutimeerap`
  (for _ (range 3)
    (`|SpawnActorFromClass` :`Class` "/Game/BluePrint/gimic/boss2gimic/timerap.timerap_C" :`SpawnTransform` (`KismetMathLibrary.MakeTransform` (`KismetMathLibrary.SelectVector` (`self.K2_GetActorLocation` (`GameplayStatics.GetPlayerCharacter` 0)) (`NavigationSystemV1.K2_GetRandomReachablePointInRadius` (`self.firstpos`) 9999.0 null null) (== (`KismetMathLibrary.RandomIntegerInRange` 0 8) 8))) :`CollisionHandlingOverride` "AlwaysSpawn" :`TransformScaleMethod` "MultiplyWithRoot" :`AoEDamage` 200.0 :`Size` 20.0 :`SphereAoE` true :`Instigator` null)))

(fn `setcircle`
  (locals (setatari :type "Array of Integer") (hontonoatari :type "Array of Integer"))
  (bind _setatari (`local.setatari`))
  (bind _hontonoatari (`local.hontonoatari`))
  (for _index (range 4)
    (`KismetArrayLibrary.Array_Add` _setatari _index))
  (for _index_2 (range 4)
    (`KismetArrayLibrary.Array_Add` _hontonoatari (`|GetArrayItem` _setatari _index_2)))
  (`KismetArrayLibrary.Array_Shuffle` _hontonoatari)
  (for _index_3 (range 4)
    (bind _returnvalue (`KismetMathLibrary.Conv_RotatorToVector` (`KismetMathLibrary.MakeRotator` 0.0 0.0 (`KismetMathLibrary.Conv_IntToDouble` (* _index_3 45)))))
    (bind _returnvalue_2 (== (`|GetArrayItem` (`local.hontonoatari`)) _index_3))
    (`self.maketimerAoE` _returnvalue 0.0 (`KismetMathLibrary.SelectFloat` 0.2 2.0 _returnvalue_2) 0.0 false 15.0)
    (bind _returnvalue_3 (`NiagaraFunctionLibrary.SpawnSystemAtLocation` "/Game/effect/tekinokougeki/clock.clock" (+ (* _returnvalue 2000) (0.0 0.0 1000.0)) (struct :`Yaw` 135.0)))
    (`PrimitiveComponent.CreateDynamicMaterialInstance` _returnvalue_3 0 "/Game/Material/clockmat.clockmat" "None")
    (`FXSystemComponent.SetFloatParameter` _returnvalue_3 "float" (* (`KismetMathLibrary.SelectFloat` 1.0 3.0 _returnvalue_2) 1.0))
    (message `AudioParameterControllerInterface.SetFloatParameter` _returnvalue_3 "time" -6.0)))

(fn `UserConstructionScript`
  (`parent.UserConstructionScript`))