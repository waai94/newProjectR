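; Fire magic actor Blueprint that inherits its core behavior from a parent class.
; On BeginPlay it runs the parent logic, plays a fire magic sound at its location, then calls Movetotarget.
; Tick and construction only forward to the parent, and the overlap event is disabled.
; Unconnected leftover nodes would spawn a Stunimpact particle system and set its position parameter, but never run.
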(event `self.ReceiveBeginPlay`
  (`parent.ReceiveBeginPlay`)
  (`GameplayStatics.PlaySoundAtLocation` "/Game/Sound/maou_se_magic_fire01.maou_se_magic_fire01" (`self.K2_GetActorLocation`) (struct) 1.0 1.0 0.0 null null null null)
  (`self.movetotarget`))

(event `self.ReceiveTick`
  (params (DeltaSeconds :type "Float (single-precision)"))
  (`parent.ReceiveTick` DeltaSeconds))

(fn `UserConstructionScript`
  (`parent.UserConstructionScript`))