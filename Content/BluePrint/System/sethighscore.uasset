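; High-score helper functions that rank and record times in the game instance's Highscore array, where a lower time is better.
; Isthishighscore stops at the first stored time that the new one matches or beats, returning a high-score flag and that array index as the rank.
; Setsocre converts a one-based rank back to an index and overwrites that entry with player, date and time, without shifting lower entries.
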(fn `isthishighscore`
  (params (NewParam :type "Float (double-precision)"))
  (returns (highscore :type Boolean) (junni :type Integer))
  (locals (nowscore :type "Float (double-precision)") (ishigh :type Boolean))
  (bind _asinstance (cast `/Game/BluePrint/System/instance` (`GameplayStatics.GetGameInstance` null)))
  (set `local.nowscore` NewParam)
  (for (_array_element _array_index) (`/Game/BluePrint/System/instance.highscore` _asinstance)
    (if (<= (`local.nowscore`) (`.Time_6_660E46294B9C28F6E3A3D8A3BEE954B5` (break `/Game/BluePrint/kouzoutai/scorearray` _array_element)))
      (set `local.ishigh` true)
      (break)))
  (return (`local.ishigh`) _array_index))

(fn `setsocre`
  (params (NewParam :type Integer) (playername :type Text) (date :type String) (time :type "Float (double-precision)"))
  ;[1 1 1] プラス１を戻す
  (bind _asinstance (cast `/Game/BluePrint/System/instance` (`GameplayStatics.GetGameInstance` null)))
  (`KismetArrayLibrary.Array_Set` (`/Game/BluePrint/System/instance.highscore` _asinstance) (- NewParam 1) (make `/Game/BluePrint/kouzoutai/scorearray` time playername 0 0 0 date)))