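; Procedural floor generator, apparently for a mystery-dungeon style level, that builds a tile map at BeginPlay.
; Husigi is a flattened Tate×Yoko integer grid, where Sixteen marks evenly spaced room centres and stamps square rooms around them.
; Createashiba then spawns an Ashiba actor per cell, 400 units apart, passing its cell value.
; Alternative generators go uncalled here: random split lines (Bunkatu), area filling (Area) and pole-toppling maze (Boudaoshi).
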(event `self.ReceiveBeginPlay`
  (for _ (range (+ (* (`self.tate`) (`self.yoko`)) 1))
    (`KismetArrayLibrary.Array_Add` (`self.husigi`)))
  (`self.sixteen`)
  (`self.createashiba`))

(fn `area`
  (locals (firstpos :type Integer) (selectedpos :type Integer) (looped :type Integer) (todayloop :type Integer) (additional :type Integer) (moreadditional :type Integer) (tateloop :type Integer))
  (bind _husigi (`self.husigi`))
  (bind _tateloop (`local.tateloop`))
  (bind _selectedpos (`local.selectedpos`))
  (bind _husigi_2 (`self.husigi`))
  (bind _selectedpos_2 (`local.selectedpos`))
  (bind _yoko (`self.yoko`))
  (bind _returnvalue (< _selectedpos (+ (`local.firstpos`) (`self.yoko`))))
  (bind _returnvalue_2 (== (`|GetArrayItem` _husigi_2 (+ _selectedpos 1)) 0))
  (for _array_element (`self.tatebunkatulo`)
    (set `local.additional` (* _yoko 3))
    (set `local.todayloop` (`KismetMathLibrary.RandomIntegerInRange` 3 5))
    (bind _returnvalue_3 (+ _array_element (`local.additional`) 0))
    (set `local.firstpos` _returnvalue_3)
    (bind _returnvalue_4 (+ _array_element (`local.moreadditional`) (`local.additional`) 1))
    (while (and (== (`|GetArrayItem` _husigi _returnvalue_4) 0) (== (`|GetArrayItem` _husigi (+ _returnvalue_4 (* _yoko 1))) 0) (<= (`local.tateloop`) 6))
      (for _index (range (+ (`local.todayloop`) 1))
        (bind _output_get (set `local.firstpos` _returnvalue_3))
        (bind _output_get_2 (set `local.selectedpos` (+ _output_get (`KismetMathLibrary.RandomIntegerInRange` 3 6))))
        (`KismetArrayLibrary.Array_Set` _husigi_2 _output_get_2 3)
        (set `local.looped` 0)
        (while (and _returnvalue_2 _returnvalue true)
          (`KismetArrayLibrary.Array_Set` _husigi_2 _selectedpos_2 2)
          (set `local.selectedpos` (+ _selectedpos_2 1))
          (set `local.looped` (+ (`local.looped`) 1)))
        (`KismetArrayLibrary.Array_Set` _husigi_2 _selectedpos_2 3)
        (`/Game/BluePrint/System/logs.printlogs` (`KismetStringLibrary.Concat_StrStr` "Cause :::: " "Looped is" (`KismetStringLibrary.Conv_BoolToString` (<= (`local.todayloop`) (`local.looped`))) "   Is 0  " (`KismetStringLibrary.Conv_BoolToString` _returnvalue_2) "  Lengh out  " (`KismetStringLibrary.Conv_BoolToString` _returnvalue)) "NewEnumerator3" true true 20.0))
      (set `local.moreadditional` (* _yoko _index))
      (set `local.tateloop` (+ _tateloop 1)))
    (`/Game/BluePrint/System/logs.printlogs` (`KismetStringLibrary.Conv_IntToString` _tateloop))))

(fn `boudaoshi`
  (locals (first :type Integer) (isnuri :type Boolean) (random :type Integer :default 0) (floorsize :type Integer) (heya :type Integer))
  (bind _yoko (`self.yoko`))
  (bind _yokobunkatulo (`self.yokobunkatulo`))
  (bind _floorsize (`local.floorsize`))
  (bind _tate (`self.tate`))
  (bind _husigi (`self.husigi`))
  (bind _husigi_2 (`self.husigi`))
  (bind _husigi_3 (`self.husigi`))
  (bind _isnuri (`local.isnuri`))
  (bind _yokobunkatulo_2 (`self.yokobunkatulo`))
  (bind _returnvalue (- 0 _floorsize))
  (`|ExecutionSequence`
    (:`then_0`
      (set `local.first` (+ _yoko 1))
      (for _index (range _tate)
        (set `local.isnuri` (not _isnuri))
        (for _index_2 (range _yoko)
          (`/Engine/EditorBlueprintResources/StandardMacros.FlipFlop`
            (:`A`
              (if _isnuri
                (bind _returnvalue_2 (+ _index_2 (* _index _tate)))
                (`KismetArrayLibrary.Array_Set` (`self.husigi`) _returnvalue_2 3)
                (`KismetArrayLibrary.Array_Add` (`self.yokobunkatulo`) _returnvalue_2)))
            (:`B`
              _))
          (set `local.first` (+ 0 2)))))
    (:`then_1`
      (for _ (range (+ (/ (`KismetArrayLibrary.Array_Length` _yokobunkatulo_2) 4) 1))
        (set `local.random` (`.OutIndex` (`KismetArrayLibrary.Array_Random` _yokobunkatulo_2)))
        (for _index_3 (range -1 2)
          (bind _output (`|GetArrayItem` _yokobunkatulo (+ (`local.random`) _index_3)))
          (`KismetArrayLibrary.Array_Set` (`self.husigi`) _output)
          (`KismetArrayLibrary.Array_Remove` _yokobunkatulo _output))))
    (:`then_2`
      (for _index_4 (range 8)
        (set `local.random` (`.OutIndex` (`KismetArrayLibrary.Array_Random` (`self.husigi`))))
        (set `local.floorsize` (`KismetMathLibrary.RandomIntegerInRange` 3 8))
        (for _index_5 (range _returnvalue (+ _floorsize 1))
          (for _index_6 (range _returnvalue (+ _floorsize 1))
            (`KismetArrayLibrary.Array_Set` (`self.husigi`) (+ (`local.random`) _index_6 (* (`self.yoko`) _index_5)) (+ _index_4 4))))))
    (:`then_3`
      (for _array_element (`self.yokobunkatulo`)
        (switch `int` (`KismetMathLibrary.RandomIntegerInRange` 0 2)
          (:`0`
            (bind _returnvalue_3 (+ _array_element 1))
            (if (== (`|GetArrayItem` _husigi_2 _returnvalue_3) 0)
              (`KismetArrayLibrary.Array_Set` _husigi_2 _returnvalue_3 2)))
          (:`1`
            (bind _returnvalue_4 (+ _array_element -1))
            (if (== (`|GetArrayItem` _husigi_3 _returnvalue_4) 0)
              (`KismetArrayLibrary.Array_Set` _husigi_3 _returnvalue_4 2)))
          (:`2`
            (bind _returnvalue_5 (+ _array_element (`self.yoko`)))
            (if (== (`|GetArrayItem` _husigi _returnvalue_5) 0)
              (`KismetArrayLibrary.Array_Set` _husigi _returnvalue_5 2))))))))

(fn `bunkatu`
  (locals (startpoint :type Integer) (pointer :type Integer))
  (`|ExecutionSequence`
    (:`then_0`
      (bind _last (`self.tatebunkatu` 8))
      (bind _output_get (set `local.startpoint` _last))
      (for _ (range 3)
        (bind _last_2 (`self.tatebunkatu` _output_get))
        (set `local.startpoint` _last_2)))
    (:`then_1`
      (for _ (range 4)
        (`self.yokobunkatu` 0 (`KismetArrayLibrary.Array_Random` (`self.tatebunkatulo`)))))))

(fn `createashiba`
  (locals (NewLocalVar :type "Vector Structure"))
  (bind _newlocalvar (`local.NewLocalVar`))
  (for _ (range (`self.tate`))
    (for _ (range (`self.yoko`))
      (`|SpawnActorFromClass` "/Game/BluePrint/System/ashiba.ashiba_C" (`KismetMathLibrary.MakeTransform` (`local.NewLocalVar`)) "AlwaysSpawn" "MultiplyWithRoot" null (`|GetArrayItem` (`self.husigi`) (`self.all`)) null)
      (set `local.NewLocalVar` (+ (`local.NewLocalVar`) (0.0 400.0 0.0)))
      (set `self.all` (+ (`self.all`) 1)))
    (set `local.NewLocalVar` (+ _newlocalvar (400.0 0.0 0.0)))
    (set `local.NewLocalVar` (`KismetMathLibrary.MakeVector` (.x _newlocalvar)))))

(fn `sixteen`
  (locals (loopin :type Integer) (floorsiz :type Integer))
  (bind _yoko (`self.yoko`))
  (bind _loopin (`local.loopin`))
  (bind _floorsiz (`local.floorsiz`))
  (bind _returnvalue (/ _yoko 5))
  (`|ExecutionSequence`
    (:`then_0`
      ;[1 1 1] 部屋の中央を取得
      (for _index (range (`self.tate`))
        (for _index_2 (range _yoko)
          (if (and (== (mod _index _returnvalue) 0) (== (mod _index_2 _returnvalue) 0))
            (`KismetArrayLibrary.Array_Set` (`self.husigi`) _loopin 2)
            (`KismetArrayLibrary.Array_Add` (`self.tatebunkatulo`) _loopin)
            (else
              (set `local.loopin` (+ _loopin 1)))))))
    (:`then_2`
      (set `local.floorsiz` 2)
      (for _array_element (`self.tatebunkatulo`)
        (for _index_3 (range -2 3)
          (for _index_4 (range (- 0 _floorsiz) (+ _floorsiz 1))
            (`KismetArrayLibrary.Array_Set` (`self.husigi`) (+ _array_element _index_4 (* (`self.yoko`) _index_3)) 3)))))
    (:`then_3`
      (for _ (range (+ (/ (`KismetArrayLibrary.Array_Length` (`self.tatebunkatulo`)) 3) 1))
        _))))

(fn `tatebunkatu`
  (params (first :type Integer))
  (returns (last :type Integer))
  (locals (startpoint :type Integer) (pointer :type Integer))
  (bind _yoko (`self.yoko`))
  (bind _startpoint (`local.startpoint`))
  (bind _startpoint_2 (`local.startpoint`))
  (bind _output_get (set `local.startpoint` (`KismetMathLibrary.RandomIntegerInRange` (+ first 7) (+ first 14))))
  (if (< _output_get _yoko)
    (`KismetArrayLibrary.Array_Set` (`self.husigi`) _output_get 1)
    (set `local.pointer` (+ _startpoint_2 (`self.yoko`)))
    (while (and (== (`|GetArrayItem` (`self.husigi`) (`local.pointer`)) 0) (< (`local.pointer`) (+ _startpoint_2 (* (`self.tate`) _yoko))))
      (`KismetArrayLibrary.Array_Set` (`self.husigi`) (`local.pointer`) 1)
      (set `local.pointer` (+ (`local.pointer`) (`self.yoko`))))
    (`KismetArrayLibrary.Array_Add` (`self.tatebunkatulo`) _startpoint)
    (return (+ _startpoint 0))))

(fn `UserConstructionScript`)

(fn `yokobunkatu`
  (params (first :type Integer) (additional :type Integer))
  (returns (last :type Integer))
  (locals (startpoint :type Integer) (pointer :type Integer))
  (bind _yoko (`self.yoko`))
  (bind _startpoint (`local.startpoint`))
  (bind _startpoint_2 (`local.startpoint`))
  (bind _output_get (set `local.startpoint` (+ (* (`self.yoko`) (`KismetMathLibrary.RandomIntegerInRange` 5 (- (`self.tate`) 5))) additional)))
  (if (< _output_get (* (`self.tate`) _yoko))
    (`KismetArrayLibrary.Array_Set` (`self.husigi`) _output_get 4)
    (set `local.pointer` (+ _startpoint_2 1))
    (while (and (== (`|GetArrayItem` (`self.husigi`) (`local.pointer`)) 0) (< (`local.pointer`) (+ _startpoint_2 _yoko)))
      (`KismetArrayLibrary.Array_Set` (`self.husigi`) (`local.pointer`) 4)
      (set `local.pointer` (+ (`local.pointer`) 1)))
    (`KismetArrayLibrary.Array_Add` (`self.yokobunkatulo`) _startpoint)
    (return _startpoint)))