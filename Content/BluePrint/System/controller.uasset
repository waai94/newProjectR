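; Player controller Blueprint that toggles the pause menu when the option input action starts.
; The input casts the game mode to Game and skips the toggle if the game is over.
; A FlipFlop drives SetGamePaused, creating a Pause widget on the viewport when pausing and removing it, if valid, on resume.
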(event `/Game/BluePrint/System/system.optionset`
  (if (not (`/Game/BluePrint/System/Game.gameisover` (stale `EnhancedInput|/Game/ThirdPerson/Input/Actions/option` _asgame))) :!label _label
    (bind _isa (`/Engine/EditorBlueprintResources/StandardMacros.FlipFlop`)
      (:`A`
        (`|ExecutionSequence`
          (:`then_0`
            (`GameplayStatics.SetGamePaused` _isa :!label _label_2))
          (:`then_1`
            (bind _returnvalue (`|CreateWidget` "/Game/Widget/pause.pause_C"))
            (`UserWidget.AddToViewport` _returnvalue 0))))
      (:`B`
        (`|ExecutionSequence`
          (:`then_0`
            (goto _label_2))
          (:`then_1`
            (`/Engine/EditorBlueprintResources/StandardMacros.IsValid` _returnvalue
              (:`Is Valid`
                (`Widget.RemoveFromParent` _returnvalue)))))))))

(event `EnhancedInput|/Game/ThirdPerson/Input/Actions/option`
  (params (ActionValue :type Boolean) (ElapsedSeconds :type "Float (double-precision)") (TriggeredSeconds :type "Float (double-precision)") (InputAction :type "InputAction Object Reference" :default "/Game/ThirdPerson/Input/Actions/option.option"))
  (:`Started`
    (bind _asgame (cast `/Game/BluePrint/System/Game` (`GameplayStatics.GetGameMode`)))
    (goto _label)))

(fn `UserConstructionScript`)