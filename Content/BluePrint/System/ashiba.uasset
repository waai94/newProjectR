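; Foothold (ashiba) actor that restarts the current level when the player touches it while its Kaidan flag is set.
; Three seconds after BeginPlay it creates a dynamic material on the Cube, tinting it red if Kaidan is set and white otherwise, via a five-color Select on Mybango.
; Box overlap casts to Player, then reopens the level by name if flagged.
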(event `self.ReceiveBeginPlay`
  (bind _kaidan (`self.kaidan`))
  (`KismetSystemLibrary.Delay` 3.0)
  (bind _returnvalue (`PrimitiveComponent.CreateDynamicMaterialInstance` (`self.Cube`) 0 "/Game/Material/ashibamat.ashibamat" "None"))
  (set `self.mybango` (`KismetMathLibrary.SelectInt` 2 0 _kaidan))
  (if _kaidan
    (`/Game/BluePrint/System/logs.printlogs` "adw" "NewEnumerator5"))
  (`MaterialInstanceDynamic.SetVectorParameterValue` _returnvalue "Param" (select `int` (`self.mybango`) :`0` (struct :`R` 1.0 :`G` 1.0 :`B` 1.0 :`A` 1.0) :`1` (struct :`G` 0.231424 :`B` 1.0 :`A` 1.0) :`2` (struct :`R` 1.0 :`B` 0.007519 :`A` 1.0) :`3` (struct :`R` 1.0 :`G` 0.775803 :`A` 1.0) :`4` (struct :`R` 0.260425 :`G` 1.0 :`A` 1.0) :!type "LinearColor Structure")))

(event `self.Box.OnComponentBeginOverlap`
  (params (OverlappedComponent :type "PrimitiveComponent Object Reference") (OtherActor :type "Actor Object Reference") (OtherComp :type "PrimitiveComponent Object Reference") (OtherBodyIndex :type Integer) (bFromSweep :type Boolean) (SweepResult :type "HitResult Structure (by ref)"))
  (cast `/Game/BluePrint/CharacterBluePrint/Player` OtherActor)
  (if (`self.kaidan`)
    (bind _returnvalue (`GameplayStatics.GetCurrentLevelName` true))
    (`GameplayStatics.OpenLevel` (`KismetStringLibrary.Conv_StringToName` _returnvalue))))

(fn `UserConstructionScript`)