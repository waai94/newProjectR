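; Button-prompt lookup that turns a game action into the input label text for the selected display scheme.
; Findhyouki reads the Hyouki (notation) setting from the game instance and switches on the action: skills, modifier, dodge, movement, item select or AA.
; Each case selects the matching keyboard, DualShock, Xbox or Switch label and returns it.
; Skill1button is an empty stub.
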(fn `findhyouki`
  (params (button :type "/Game/BluePrint/rekkyo/tukaubotan Enum" :default "NewEnumerator0"))
  (returns (return :type String))
  (locals (gameinstance :type "GameInstance Object Reference") (triger :type String) (hyouki :type "/Game/BluePrint/rekkyo/gamehyouki Enum" :default "NewEnumerator0"))
  (bind _hyouki (`local.hyouki`))
  (bind _hyouki_2 (`local.hyouki`))
  (`|ExecutionSequence`
    (:`then_0`
      (bind _output_get (set `local.gameinstance` (`GameplayStatics.GetGameInstance` null)))
      (bind _asinstance (cast `/Game/BluePrint/System/instance` _output_get))
      (set `local.hyouki` (`/Game/BluePrint/System/instance.hyouki` _asinstance))
      (switch `/Game/BluePrint/rekkyo/tukaubotan` button
        (:`NewEnumerator0`
          (set `local.triger` (select `/Game/BluePrint/rekkyo/gamehyouki` (`local.hyouki`) :`NewEnumerator0` "Q" :`NewEnumerator1` "□" :`NewEnumerator2` "X" :`NewEnumerator3` "Y")))
        (:`NewEnumerator1`
          (set `local.triger` (select `/Game/BluePrint/rekkyo/gamehyouki` (`local.hyouki`) :`NewEnumerator0` "E" :`NewEnumerator1` "△" :`NewEnumerator2` "Y" :`NewEnumerator3` "X")))
        (:`NewEnumerator2`
          (set `local.triger` (select `/Game/BluePrint/rekkyo/gamehyouki` (`local.hyouki`) :`NewEnumerator0` "R" :`NewEnumerator1` "〇" :`NewEnumerator2` "B" :`NewEnumerator3` "A")))
        (:`NewEnumerator3`
          (set `local.triger` (select `/Game/BluePrint/rekkyo/gamehyouki` _hyouki_2 :`NewEnumerator0` "Shift" :`NewEnumerator1` "L1" :`NewEnumerator2` "LB" :`NewEnumerator3` "L")))
        (:`NewEnumerator4`
          (set `local.triger` (select `/Game/BluePrint/rekkyo/gamehyouki` _hyouki_2 :`NewEnumerator0` "Ctrl" :`NewEnumerator1` "R2" :`NewEnumerator2` "RT" :`NewEnumerator3` "ZR")))
        (:`NewEnumerator5`
          (set `local.triger` (select `/Game/BluePrint/rekkyo/gamehyouki` _hyouki_2 :`NewEnumerator0` "WASD" :`NewEnumerator1` "LS" :`NewEnumerator2` "L" :`NewEnumerator3` "L")))
        (:`NewEnumerator6`
          (set `local.triger` (select `/Game/BluePrint/rekkyo/gamehyouki` _hyouki :`NewEnumerator0` "1-3" :`NewEnumerator1` "十字左右" :`NewEnumerator2` "十字左右" :`NewEnumerator3` "十字左右")))
        (:`NewEnumerator8`
          (set `local.triger` (select `/Game/BluePrint/rekkyo/gamehyouki` _hyouki :`NewEnumerator0` "Space" :`NewEnumerator1` "×" :`NewEnumerator2` "A" :`NewEnumerator3` "B")))))
    (:`then_1`
      (return (`local.triger`)))))

(fn `skill1button`)