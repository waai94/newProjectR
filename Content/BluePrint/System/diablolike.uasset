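; Procedural dungeon generator that lays out a Diablo-like floor of Ashiba (foothold) tiles at BeginPlay.
; Tile runs a grid random walk, moving the actor itself as a probe and using its Box overlap to find free neighbouring cells.
; When boxed in, Findnewlocate branches from a random existing tile.
; Afterwards it teleports the player onto the first tile and flags the last as Kaidan (stairs); the enemy-spawning and Overloop regeneration calls are disconnected.
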(event `self.ReceiveBeginPlay`
  (`self.tile`))

(event `spawnplayer`
  (bind _returnvalue (`GameplayStatics.GetPlayerCharacter` 0))
  (`KismetSystemLibrary.RetriggerableDelay` 0.1)
  (`/Engine/EditorBlueprintResources/StandardMacros.DoOnce` false
    (:`Completed`
      (bind _outactors (`GameplayStatics.GetAllActorsOfClass` "/Game/BluePrint/System/ashiba.ashiba_C"))
      (`/Engine/EditorBlueprintResources/StandardMacros.IsValid` _returnvalue
        (:`Is Valid`
          (`self.K2_SetActorLocation` _returnvalue (+ (`self.K2_GetActorLocation` (`|GetArrayItem` _outactors)) (0.0 0.0 200.0)) false false))
        (:`Is Not Valid`
          _))
      (bind _output_get (set `self.NewVar` (`|GetArrayItem` _outactors (`KismetArrayLibrary.Array_LastIndex` _outactors))))
      (`/Engine/EditorBlueprintResources/StandardMacros.IsValid` _output_get
        (:`Is Valid`
          (set `/Game/BluePrint/System/ashiba.kaidan` true (`self.NewVar`)))
        (:`Is Not Valid`
          (`/Game/BluePrint/System/logs.printlogs` "No Target" "NewEnumerator1")))
      (`/Engine/EditorBlueprintResources/StandardMacros.DoOnce` false))))

(fn `findnewlocate`
  (locals (ashibaall :type "Array of /Game/BluePrint/System/ashiba Object Reference") (check :type "/Game/BluePrint/System/ashiba Object Reference"))
  (bind _outactors (`GameplayStatics.GetAllActorsOfClass` "/Game/BluePrint/System/ashiba.ashiba_C"))
  (bind _output_get (set `local.ashibaall` _outactors))
  (set `local.check` (`KismetArrayLibrary.Array_Random` _output_get))
  (for _index (range 4)
    (`self.K2_SetActorLocation` (+ (`self.K2_GetActorLocation` (`local.check`)) (* (select `int` _index :`0` (1.0 0.0 0.0) :`1` (0.0 1.0 0.0) :`2` (-1.0 0.0 0.0) :`3` (0.0 -1.0 0.0) :!type "Vector Structure") (`self.ookisa`))) false true)
    (if (== (`KismetArrayLibrary.Array_Length` (`PrimitiveComponent.GetOverlappingActors` (`self.Box`) "/Game/BluePrint/System/ashiba.ashiba_C")) 0)
      (set `self.locate` (`self.K2_GetActorLocation`))
      (break))))

(fn `maketile`
  (bind _locate (`self.locate`))
  (bind _kaidan (`self.kaidan`))
  (`|SpawnActorFromClass` "/Game/BluePrint/System/ashiba.ashiba_C" (`KismetMathLibrary.MakeTransform` (`KismetMathLibrary.SelectVector` (+ _locate (`KismetMathLibrary.MakeVector` 0.0 0.0 (/ (`self.ookisa`) 2.0))) _locate _kaidan) (`KismetMathLibrary.SelectRotator` (`KismetMathLibrary.MakeRotator` 0.0 (`KismetMathLibrary.SelectFloat` 45.0 -45.0 (> (`self.kaisou`) 0)) (select `int` (`self.houkou`) :`0` 0.0 :`1` 90.0 :`2` 180.0 :`3` -90.0 :!type "Float (single-precision)")) (struct) _kaidan) (0.78 0.78 0.78)) "Undefined" "MultiplyWithRoot" null 0 false null)
  (set `self.locate` (+ (`self.locate`) (`KismetMathLibrary.MakeVector` 0.0 0.0 (`KismetMathLibrary.SelectFloat` (`self.ookisa`) 0.0 (`self.kaidan`))))))

(fn `overloop`
  (set `self.finished` false)
  (bind _output_get (set `self.overloopedtime` (+ (`self.overloopedtime`) 1)))
  (if (<= (`self.tileloop`) 120)
    (bind _outactors (`GameplayStatics.GetAllActorsOfClass` "/Game/BluePrint/System/ashiba.ashiba_C"))
    (for _array_element _outactors
      (`self.K2_DestroyActor` _array_element))
    (if (>= _output_get 30)
      (`KismetSystemLibrary.K2_SetTimer` null "Tile" 0.1)
      (else
        (`self.tile`)))
    (else
      (set `self.finished` true))))

(fn `spawn`)

(fn `tile`
  (bind _returnvalue (`KismetMathLibrary.RandomIntegerInRange` 0 3))
  (bind _returnvalue_2 (< (`self.looped`) (`self.max`)))
  (set `self.locate` (0.0 0.0 0.0))
  (set `self.tileloop` 0)
  (set `self.finished` false)
  (for _ (range (+ (`self.kaisuu`) 1))
    (if (not (`self.finished`))
      (set `self.tileloop` 0)
      (`self.maketile`)
      (if (`self.kaidan`)
        (set `self.newhoukou` (`self.houkou`))
        (bind _output_get (set `self.houkou` (`self.newhoukou`) :!label _label))
        (set `self.locate` (+ (`self.locate`) (* (select `int` _output_get :`0` (1.0 0.0 0.0) :`1` (0.0 1.0 0.0) :`2` (-1.0 0.0 0.0) :`3` (0.0 -1.0 0.0) :!type "Vector Structure") (`self.ookisa`))))
        (set `self.kaidan` false)
        (if (== (`KismetMathLibrary.RandomIntegerInRange` 0 4) 0)
          _)
        (else
          (set `self.newhoukou` _returnvalue)
          (`self.K2_SetActorLocation` (+ (`self.locate`) (* (select `int` (`self.newhoukou`) :`0` (1.0 0.0 0.0) :`1` (0.0 1.0 0.0) :`2` (-1.0 0.0 0.0) :`3` (0.0 -1.0 0.0) :!type "Vector Structure") (`self.ookisa`))) true)
          (set `self.looped` 0)
          (while (and _returnvalue_2 (not (== (`KismetArrayLibrary.Array_Length` (`PrimitiveComponent.GetOverlappingActors` (`self.Box`) "/Script/Engine.Actor")) 0)))
            (bind _output_get_2 (set `self.newhoukou` _returnvalue))
            (`self.K2_SetActorLocation` (+ (`self.locate`) (* (select `int` _output_get_2 :`0` (1.0 0.0 0.0) :`1` (0.0 1.0 0.0) :`2` (-1.0 0.0 0.0) :`3` (0.0 -1.0 0.0) :!type "Vector Structure") (`self.ookisa`))))
            (set `self.looped` (+ (`self.looped`) 1))
            (if (> (`self.looped`) (`self.max`))
              (`self.findnewlocate`)))
          (if _returnvalue_2
            (goto _label)
            (else
              (`self.findnewlocate`)))))))
  (`/Game/BluePrint/System/logs.printlogs` "completed!" "NewEnumerator3")
  (`self.spawnplayer`))

(fn `UserConstructionScript`)