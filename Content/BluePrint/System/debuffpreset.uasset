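; Builds a status-effect (Joutailist) struct for buffs and debuffs such as stun, slow, damage/heal over time and invincibility.
; With Preset on, Select nodes keyed on the effect type supply duration, strength, Japanese name and description, and material, with only VulnerabilityUp stackable.
; Otherwise it passes caller values through.
; Faster and AttackDamage have blank presets, and an empty-description fallback is left unconnected.
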(fn `presetdebuff`
  (params (joutai :type "/Game/BluePrint/rekkyo/joutaiijou Enum" :default "NewEnumerator0") (time :type "Float (double-precision)") (NewParam1 :type "Actor Object Reference") (strong :type "Float (double-precision)") (name :type Text) (isstack :type Boolean) (material :type "MaterialInstance Object Reference") (NewParam2 :type Text) (preset :type Boolean))
  (returns (NewParam :type "/Game/BluePrint/kouzoutai/joutailist Structure"))
  (return (select `bool` preset :`false` (make `/Game/BluePrint/kouzoutai/joutailist` joutai time NewParam1 strong name isstack material NewParam2) :`true` (make `/Game/BluePrint/kouzoutai/joutailist` joutai (select `/Game/BluePrint/rekkyo/joutaiijou` joutai :`NewEnumerator0` 3.0 :`NewEnumerator1` 3.0 :`NewEnumerator2` 3.0 :`NewEnumerator3` 3.0 :`NewEnumerator4` 30.0 :`NewEnumerator5` 30.0 :`NewEnumerator6` 60.0 :`NewEnumerator7` 3.0) NewParam1 (select `/Game/BluePrint/rekkyo/joutaiijou` joutai :`NewEnumerator0` 1.0 :`NewEnumerator1` 1.0 :`NewEnumerator2` 0.1 :`NewEnumerator3` 1.0 :`NewEnumerator4` 30.0 :`NewEnumerator5` 30.0 :`NewEnumerator6` 0.5) (select `/Game/BluePrint/rekkyo/joutaiijou` joutai :`NewEnumerator0` "スタン" :`NewEnumerator1` "スネア" :`NewEnumerator2` "恐怖" :`NewEnumerator3` "スロウ" :`NewEnumerator4` "出血" :`NewEnumerator5` "リジェネ" :`NewEnumerator6` "被ダメージ上昇" :`NewEnumerator7` "無敵" :!type "Text") (`|EnumEquality` joutai "NewEnumerator6") (select `/Game/BluePrint/rekkyo/joutaiijou` joutai :`NewEnumerator0` "/Game/Texture/icons/debuff/stun.stun" :`NewEnumerator1` "/Game/Texture/icons/debuff/stun.stun" :`NewEnumerator2` "/Game/Texture/icons/debuff/stun.stun" :`NewEnumerator3` "/Game/Texture/icons/debuff/stun.stun" :`NewEnumerator4` "/Game/Texture/icons/debuff/poisondebuff.poisondebuff" :`NewEnumerator5` "/Game/Texture/icons/regene.regene" :`NewEnumerator6` "/Game/Texture/icons/debuff/vitup.vitup" :!type "MaterialInstance Object Reference") (select `/Game/BluePrint/rekkyo/joutaiijou` joutai :`NewEnumerator0` "行動できない状態。" :`NewEnumerator1` "移動できない状態。" :`NewEnumerator2` "恐怖により体が言うことを聞かない！" :`NewEnumerator3` "行動速度が低下した状態。" :`NewEnumerator4` "継続的にダメージを受けている。" :`NewEnumerator5` "継続的に回復を受けている状態。" :`NewEnumerator6` "被ダメージが上昇している状態。" :`NewEnumerator7` "攻撃を一切受け付けない状態。" :!type "Text")))))