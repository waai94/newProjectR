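; Area damage gimmick that deals distance-attenuated damage (kyorigensui) to actors overlapping its sphere, then destroys itself.
; BeginPlay waits for Taiki, then calls the Ensyutu event, which is empty here; nothing in this graph calls damage.
; The damage event scales Basedamage by sphere scale over distance, clamped to a minimum factor, logs the factor, and sends it via GoingdamageMessage.
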(event `self.ReceiveBeginPlay`
  (`KismetSystemLibrary.Delay` (`self.taiki`))
  (`self.ensyutu`))

(event `ensyutu`)

(event `damage`
  (for _array_element (`PrimitiveComponent.GetOverlappingActors` (`self.Sphere`) "/Script/Engine.Actor")
    (`/Engine/EditorBlueprintResources/StandardMacros.IsValid` _array_element
      (:`Is Valid`
        (bind _returnvalue (/ (* (.x (`SceneComponent.K2_GetComponentScale` (`self.Sphere`))) 32.0) (+ (`self.GetDistanceTo` _array_element self) 0.01) 3.0))
        (`/Game/BluePrint/System/logs.printlogs` (`KismetStringLibrary.Conv_DoubleToString` _returnvalue) "NewEnumerator3")
        (message `/Game/BluePrint/System/damagekankei.goingdamage` _array_element (* (`self.basedamage`) (`KismetMathLibrary.FClamp` _returnvalue 0.1 99999.0)) false (struct) self 0.0 null 0.0))))
  (`self.K2_DestroyActor`))

(event `self.ReceiveTick`
  (params (DeltaSeconds :type "Float (single-precision)")))

(fn `UserConstructionScript`)