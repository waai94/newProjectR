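; Base area-of-effect attack actor that shows a telegraph decal after a delay, hides it, then calls the empty Ensyutu hook.
; Tick grows the sphere and animates the ring's inner radius, while Huttobasu, active for knockback attacks, orients toward the player.
; The damaged event hits sphere overlaps outside the inner ring or box overlaps, applying damage, knockback and extra crowd control, then destroys the actor.
; Ringtemplete spawns ring-scaled effects.
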(event `self.ReceiveBeginPlay`
  (bind _sphereaoe (`self.SphereAoE`))
  (`KismetSystemLibrary.Delay` (`self.jobantaiki`))
  (`self.SetActorHiddenInGame` false)
  (`SceneComponent.SetHiddenInGame` (`self.Decal`) _sphereaoe false)
  (`SceneComponent.SetHiddenInGame` (`self.spheredecal`) (not _sphereaoe) false)
  (`ActorComponent.SetActive` (`self.huttobasu`) (> (`self.Knockback`) 1.0) false)
  (bind _returnvalue (`DecalComponent.CreateDynamicMaterialInstance` (`self.spheredecal`)))
  (set `self.dynamicmat` _returnvalue)
  (`KismetSystemLibrary.Delay` (`self.yochoudelay`))
  (`self.SetActorHiddenInGame` true)
  (`KismetSystemLibrary.Delay` (`self.delayed`))
  (`self.ensyutu`))

(event `ringtemplete`
  (params (SystemTemplate :type "NiagaraSystem Object Reference"))
  (bind _size (`self.Size`))
  (bind _returnvalue (`NiagaraFunctionLibrary.SpawnSystemAtLocation` SystemTemplate (`self.K2_GetActorLocation`)))
  (`FXSystemComponent.SetFloatParameter` _returnvalue "ringradius" (* _size 32.0))
  (`FXSystemComponent.SetFloatParameter` _returnvalue "ringhankei" (- 1.0 (/ (/ (`self.ringdistance`) _size) 2.0))))

(event `damaged`
  (params (fordestroy :type "Float (double-precision)"))
  (if (`self.SphereAoE`)
    (for _array_element (`PrimitiveComponent.GetOverlappingActors` (`self.Sphere`) "/Script/Engine.Actor")
      (if (or (> (/ (`KismetMathLibrary.Vector_Distance` (`self.K2_GetActorLocation`) (`self.K2_GetActorLocation` _array_element)) 32.0) (`self.ringdistance`)) (== (`self.ringdistance`) 0.0))
        (bind _newparam (`/Game/BluePrint/System/debuffpreset.presetdebuff` "NewEnumerator6" 0.0 self 0.0 "" false null "" true))
        (message `/Game/BluePrint/System/damagekankei.goingdamage` _array_element (`self.AoEDamage`) (`self.penaltyup`) _newparam self (`self.Knockback`) null 0.0)
        (`self.joutai` _array_element)))
    (`KismetSystemLibrary.Delay` fordestroy)
    (`self.K2_DestroyActor`)
    (else
      (for _array_element_2 (`PrimitiveComponent.GetOverlappingActors` (`self.Box`) "/Script/Engine.Actor")
        (bind _newparam_2 (`/Game/BluePrint/System/debuffpreset.presetdebuff` "NewEnumerator6" 60.0 self 0.5 "" false null "" true))
        (message `/Game/BluePrint/System/damagekankei.goingdamage` _array_element_2 (`self.AoEDamage`) (`self.penaltyup`) _newparam_2 self (`self.Knockback`) null 0.0)
        (`self.joutai` _array_element_2))
      (`/Game/BluePrint/System/logs.printlogs` (`KismetStringLibrary.Conv_DoubleToString` fordestroy))
      (`KismetSystemLibrary.Delay` fordestroy)
      (`self.K2_DestroyActor`))))

(event `ensyutu`)

(event `joutai`
  (params (NewParam :type "Actor Object Reference"))
  (for _array_element (`self.tuikacc`)
    (message `/Game/BluePrint/System/damagekankei.goingdamage` NewParam 0.0 true _array_element self 0.0 "/Script/Engine.DamageType" 0.0)))

(event `self.ReceiveTick`
  (params (DeltaSeconds :type "Float (single-precision)"))
  (bind _size (`self.Size`))
  (bind _sphere (`self.Sphere`))
  (bind _huttobasu (`self.huttobasu`))
  (bind _dynamicmat (`self.dynamicmat`))
  (bind _yaw (.yaw (`KismetMathLibrary.FindLookAtRotation` (`self.K2_GetActorLocation`) (`self.K2_GetActorLocation` (`GameplayStatics.GetPlayerCharacter` 0)))))
  (set `self.time` (+ (`self.time`) DeltaSeconds))
  (`FXSystemComponent.SetVectorParameter` _huttobasu "forward" (`KismetMathLibrary.GetForwardVector` (`KismetMathLibrary.MakeRotator` 0.0 0.0 (- _yaw 90.0))))
  (`FXSystemComponent.SetVectorParameter` _huttobasu "move" (`KismetMathLibrary.GetForwardVector` (`KismetMathLibrary.MakeRotator` 0.0 0.0 _yaw)))
  (if (>= (`self.time`) (`self.jobantaiki`))
    (`SceneComponent.SetWorldScale3D` _sphere (`KismetMathLibrary.VInterpTo` (`SceneComponent.K2_GetComponentScale` _sphere) (`KismetMathLibrary.MakeVector` _size _size _size) DeltaSeconds 10.0))
    (`/Engine/EditorBlueprintResources/StandardMacros.IsValid` _dynamicmat
      (:`Is Valid`
        (bind _output_get (set `self.ringsize` (`KismetMathLibrary.FInterpTo` (`self.ringsize`) (/ (/ (`self.ringdistance`) (`self.Size`)) 2.0) (`GameplayStatics.GetWorldDeltaSeconds`) 10.0)))
        (`MaterialInstanceDynamic.SetScalarParameterValue` _dynamicmat "ookisa" _output_get)))))

(fn `UserConstructionScript`)