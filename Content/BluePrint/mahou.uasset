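; Magic projectile actor that homes in on a stored TARGET and delivers damage when it arrives.
; The movetotarget event records the start location, then a timeline lerps the actor toward the target's current location each update.
; On finish it sends GoingdamageMessage with damage and critical flag to the target, then destroys itself.
; A missing or lost target is logged and the projectile is destroyed; an ApplyDamage branch is left unconnected.
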(event `movetotarget`
  (bind _target (`self.TARGET`))
  (`/Engine/EditorBlueprintResources/StandardMacros.IsValid` _target
    (:`Is Valid`
      (bind _output_get (set `self.firstlocation` (`self.K2_GetActorLocation`)))
      (bind (_direction `_新規track_0`) (`Timeline|タイムライン` :!via `PlayFromStart`)
        (:`Update`
          (`self.K2_SetActorLocation` (`KismetMathLibrary.VLerp` _output_get (`self.K2_GetActorLocation` _target) `_新規track_0`))
          (`/Engine/EditorBlueprintResources/StandardMacros.IsValid` _target
            (:`Is Not Valid`
              (`/Game/BluePrint/System/logs.printlogs` "対象がキルされた可能性があります。" "NewEnumerator1")
              (`self.K2_DestroyActor` :!label _label))))
        (:`Finished`
          (message `/Game/BluePrint/System/damagekankei.goingdamage` _target (`self.DAMAGE`) false (struct) self 0.0 null (`self.ctitical`))
          (`self.K2_DestroyActor`))))
    (:`Is Not Valid`
      (`/Game/BluePrint/System/logs.printlogs` "対象を発見できませんでした。" "NewEnumerator1")
      (goto _label))))

(fn `UserConstructionScript`)